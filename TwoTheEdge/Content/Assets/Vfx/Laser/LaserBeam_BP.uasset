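; Laser beam hazard actor that respawns any BP_Character caught by its line trace, unless that character is already respawning.
; BeginPlay sets the particle beam once between two static meshes, with an offset at the source, then fires the trace immediately and on a looping timer.
; The periodic Camera-channel trace, with debug drawing on, runs from the Box to the target mesh and does the detection; the overlap event is empty.
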(event Custom|LaserOn
  (bind _outhit (Collision|LineTraceByChannel (Transformation|GetWorldLocation (Variables|Default|GetBox)) (Transformation|GetWorldLocation (Variables|Default|GetStaticMesh1)) "TraceTypeQuery2" false 0 "ForDuration"))
  (bind _asbp_character (Utilities|Casting|CastToBP_Character (.HitActor (Collision|BreakHitResult _outhit))))
  (if (not (Variables|/Game/Blueprints/Pawns/BP_Character_New.BP_Character_C|GetRespawning _asbp_character))
    (Class|TwotheEdgeCharacter|Respawn _asbp_character)))

(event Collision|EventActorBeginOverlap
  (params (OtherActor :type Actor%20Object%20Reference)))

(event EventBeginPlay
  (bind _particlesystem (Variables|Default|GetParticleSystem))
  (Utilities|Time|SetTimerbyFunctionName 0 "LaserOn" 2.5 true)
  (Class|ParticleSystemComponent|SetBeamSourcePoint _particlesystem 0 (- (Transformation|GetWorldLocation (Variables|Default|GetStaticMesh)) (Variables|Default|GetLaserStartPlacement)))
  (Class|ParticleSystemComponent|SetBeamTargetPoint _particlesystem 0 (Transformation|GetWorldLocation (Variables|Default|GetStaticMesh1)))
  (bind _outhit (Collision|LineTraceByChannel (Transformation|GetWorldLocation (Variables|Default|GetBox)) (Transformation|GetWorldLocation (Variables|Default|GetStaticMesh1)) "TraceTypeQuery2" false 0 "ForDuration"))
  (bind _asbp_character (Utilities|Casting|CastToBP_Character (.HitActor (Collision|BreakHitResult _outhit))))
  (if (not (Variables|/Game/Blueprints/Pawns/BP_Character_New.BP_Character_C|GetRespawning _asbp_character))
    (Class|TwotheEdgeCharacter|Respawn _asbp_character)))

(fn ConstructionScript)