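; Laser beam VFX actor that stretches a particle beam between two static meshes.
; On BeginPlay it sets the beam source to the first mesh's location minus a LaserStartPlacement offset and the target to the second mesh's location, with no later updates.
; Each Tick line-traces against its Box component from the box to the second mesh, but the result is unused.
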(event EventBeginPlay
  (bind _particlesystem (Variables|Default|GetParticleSystem))
  (Class|ParticleSystemComponent|SetBeamSourcePoint _particlesystem 0 (- (Transformation|GetWorldLocation (Variables|Default|GetStaticMesh)) (Variables|Default|GetLaserStartPlacement)))
  (Class|ParticleSystemComponent|SetBeamTargetPoint _particlesystem 0 (Transformation|GetWorldLocation (Variables|Default|GetStaticMesh1))))

(event Collision|EventActorBeginOverlap
  (params (OtherActor :type Actor%20Object%20Reference)))

(event EventTick
  (params (DeltaSeconds :type Float%20%28single-precision%29))
  (Collision|LineTraceComponent (Variables|Default|GetBox) (Transformation|GetWorldLocation (Variables|Default|GetBox)) (Transformation|GetWorldLocation (Variables|Default|GetStaticMesh1)) true false false))

(fn ConstructionScript)