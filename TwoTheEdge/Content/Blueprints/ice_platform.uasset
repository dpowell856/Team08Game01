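; Ice platform actor that moves between two configurable relative locations using an InterpToMovement component.
; The construction script builds the control points from Location1 and Location2 and applies the Duration.
; BeginPlay records the starting world location and, on authority only, calls Server to activate the movement.
; Timer-based position sync, which would teleport the platform to CurrentServerLocation, is left unconnected and never runs.
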(event Custom|Server
  (Components|Activation|Activate (Variables|Default|GetInterpToMovement) false))

(event Custom|Client)

(event Custom|ClientRefresh
  (bind _interptomovement (Variables|Default|GetInterpToMovement))
  (Class|MovementComponent|MoveUpdatedComponent _interptomovement (- (Variables|Default|GetCurrentServerLocation) (Transformation|GetWorldLocation (Variables|/Script/Engine.MovementComponent|GetUpdatedComponent _interptomovement))) "0, 0, 0" false true))

(event Custom|SetCurrentLocation
  (Variables|Default|SetCurrentServerLocation (Transformation|GetWorldLocation (Variables|/Script/Engine.MovementComponent|GetUpdatedComponent (Variables|Default|GetInterpToMovement)))))

(event EventBeginPlay
  (Variables|Default|SetCurrentServerLocation (Transformation|GetWorldLocation (Variables|/Script/Engine.MovementComponent|GetUpdatedComponent (Variables|Default|GetInterpToMovement))))
  (Networking|SwitchHasAuthority
    (:Authority
      (CallFunction|Server))))

(event Collision|EventActorBeginOverlap
  (params (OtherActor :type Actor%20Object%20Reference)))

(event EventTick
  (params (DeltaSeconds :type Float%20%28single-precision%29)))

(fn ConstructionScript
  (bind _interptomovement (Variables|Default|GetInterpToMovement))
  (Variables|/Script/Engine.InterpToMovementComponent|SetControlPoints _interptomovement (Utilities|Array|MakeArray (Utilities|Struct|MakeInterpControlPoint (Variables|Default|GetLocation1) true) (Utilities|Struct|MakeInterpControlPoint (Variables|Default|GetLocation2) true)))
  (Variables|/Script/Engine.InterpToMovementComponent|SetDuration _interptomovement (Variables|Default|GetDuration)))