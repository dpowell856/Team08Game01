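; Game mode for Two The Edge that detects when every player has finished.
; On BeginPlay it starts a short looping timer that scans the GameState's PlayerArray for any TwoTheEdgePlayerState not yet marked Finished.
; When none remain, it sets GameFinished, which makes later checks do nothing, and prints a completion message.
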(event Custom|CheckIfGameFinished
  (if (not (Variables|Default|GetGameFinished))
    (Variables|Default|SetPlayersRemaining false)
    (bind _array_element (Utilities|Array|ForEachLoopwithBreak (Variables|/Script/Engine.GameStateBase|GetPlayerArray (Game|GetGameState)) :!label _label)
      (:LoopBody
        (bind _astwo_the_edge_player_state (Utilities|Casting|CastToTwoTheEdgePlayerState _array_element))
        (if (not (Variables|/Script/TwoTheEdge.TwoTheEdgePlayerState|GetFinished _astwo_the_edge_player_state))
          (Variables|Default|SetPlayersRemaining true)
          (goto _label Break)))
      (:Completed
        (if (not (Variables|Default|GetPlayersRemaining))
          (Variables|Default|SetGameFinished true)
          (Development|PrintString "Game complete!"))))))

(event EventBeginPlay
  (Utilities|Time|SetTimerbyEvent (delegate Custom|CheckIfGameFinished) 0.2 true))

(fn ConstructionScript)