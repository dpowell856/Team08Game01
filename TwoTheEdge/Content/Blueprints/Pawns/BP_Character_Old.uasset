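; Player character Blueprint (an older version, by its name) with surface-based movement, checkpoint respawn and a grenade throw.
; A looping timer sets ground friction and braking from the floor's physical surface, making ice slippery and tar sticky.
; Right mouse spawns an explosion grenade beside the mesh and launches it with velocity derived from clamped camera pitch.
; Respawn teleports the character to the last checkpoint stored in the PlayerState.
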(event Custom|UpdateGroundType
  (bind _charactermovement (Variables|Character|GetCharacterMovement))
  (bind _charactermovement_2 (Variables|Character|GetCharacterMovement))
  (bind _currentfloor (Variables|/Script/Engine.CharacterMovementComponent|GetCurrentFloor _charactermovement))
  (bind _returnvalue (Collision|GetSurfaceType (.hitresult _currentfloor)))
  (Variables|/Script/Engine.CharacterMovementComponent|SetGroundFriction _charactermovement_2 (Utilities|Select :Index _returnvalue :SurfaceType_Default 0.8 :SurfaceType1 0.1 :SurfaceType2 2.0))
  (Variables|/Script/Engine.CharacterMovementComponent|SetBrakingDecelerationWalking _charactermovement_2 (Utilities|Select :Index _returnvalue :SurfaceType_Default 1.5e+03 :SurfaceType1 0.0 :SurfaceType2 5e+03)))

(event Custom|OnRespawn_1
  (bind _astwo_the_edge_player_state (Utilities|Casting|CastToTwoTheEdgePlayerState (Variables|Default|GetPlayerState)))
  (Transformation|Teleport (.location (Variables|/Script/TwoTheEdge.TwoTheEdgePlayerState|GetLastCheckpointPos _astwo_the_edge_player_state)) (.rotation (Variables|/Script/TwoTheEdge.TwoTheEdgePlayerState|GetLastCheckpointPos _astwo_the_edge_player_state))))

(event EventBeginPlay
  (Utilities|Time|SetTimerbyFunctionName 0 "UpdateGroundType" 0.1 true))

(event Input|MouseEvents|RightMouseButton
  (params (Key :type Key%20Structure :default "None"))
  (:Pressed
    (CallFunction|GrenadeThrow)))

(fn ConstructionScript
  (Variables|Default|SetExtraMovement self (Variables|Default|GetExtraMovementComponent)))

(fn GrenadeThrow
  (bind _followcamera (Variables|Default|GetFollowCamera))
  (bind _mesh (Variables|Character|GetMesh))
  (bind _returnvalue (Math|Vector|GetRightVector _mesh))
  (bind _returnvalue_2 (Math|Vector|GetUpVector _mesh))
  (bind _returnvalue_3 (Transformation|GetWorldRotation _followcamera))
  (bind _returnvalue_4 (Math|Float|ClampAngle (.pitch _returnvalue_3) -5e+01 5e+01))
  (bind _returnvalue_5 (* (.z _returnvalue_2) 8e+02))
  (bind _returnvalue_6 (* _returnvalue_4 5e+01))
  (bind _returnvalue_7 (+ _returnvalue_5 _returnvalue_6))
  (bind _returnvalue_8 (Math|Float|Min(Float) _returnvalue_7 8e+02))
  (bind _returnvalue_9 (Math|Float|Max(Float) _returnvalue_8 -4e+02))
  (bind _returnvalue_10 (Math|Float|Lerp 7.5e+02 _returnvalue_9 0.5))
  (bind _returnvalue_11 (Math|Float|Max(Float) _returnvalue_10 1e+02))
  (bind _returnvalue_12 (* _returnvalue _returnvalue_11))
  (bind _returnvalue_13 (Game|SpawnActorfromClass "/Game/Blueprints/Actors/BP_ExplosionGrenade.BP_ExplosionGrenade_C" (Math|Conversions|ToTransform(Vector) (+ (+ (Transformation|GetWorldLocation _mesh) "0, 0,180.000000") (* _returnvalue 75.0))) "Undefined" 0 0))
  (Physics|SetPhysicsLinearVelocity (Variables|/Game/Blueprints/Actors/BP_ExplosionGrenade.BP_ExplosionGrenade_C|GetSphere _returnvalue_13) (Math|Vector|MakeVector (.x _returnvalue_12) (.y _returnvalue_12) _returnvalue_9) false "None") ; Adds force to the grenade
)