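; Player character Blueprint for a networked game, adding dash montage, explosive and freeze grenades, respawning and player colours.
; Grenade input requests a throw, which spawns a projectile with velocity derived from camera pitch.
; Timers set friction and braking by floor surface (ice, tar) and trigger kill-Z respawns.
; Respawn teleports to the PlayerState checkpoint between disintegrate-material fades, relaying fade-in through server calls; that material also carries the player's colour texture.
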(event Custom|UpdateGroundType
  (bind _charactermovement (Variables|Character|GetCharacterMovement))
  (bind _charactermovement_2 (Variables|Character|GetCharacterMovement))
  (bind _currentfloor (Variables|/Script/Engine.CharacterMovementComponent|GetCurrentFloor _charactermovement))
  (bind _returnvalue (Collision|GetSurfaceType (.hitresult _currentfloor)))
  (Variables|/Script/Engine.CharacterMovementComponent|SetGroundFriction _charactermovement_2 (Utilities|Select :Index _returnvalue :SurfaceType_Default 0.8 :SurfaceType1 0.1 :SurfaceType2 2.0))
  (Variables|/Script/Engine.CharacterMovementComponent|SetBrakingDecelerationWalking _charactermovement_2 (Utilities|Select :Index _returnvalue :SurfaceType_Default 1.5e+03 :SurfaceType1 0.0 :SurfaceType2 5e+03)))

(event Custom|CheckKillZServer
  (if (<= (.z (Transformation|GetWorldLocation (Variables|Default|GetCapsuleComponent))) -3e+03)
    (if (not (Variables|Default|GetRespawning))
      (Class|TwotheEdgeCharacter|Respawn))))

(event Custom|CallServer
  ;[1 1 1 1 12] Basically tells the client to tell the server to tell everyone to do fade out. It was working perfectly before, but whatever, this fixes it.
  (CallFunction|CallAll))

(event Custom|CallAll
  ;[1 1 1 1 12] Basically tells the client to tell the server to tell everyone to do fade out. It was working perfectly before, but whatever, this fixes it.
  (bind _fadein (Timeline|FadeIn ReverseFromEnd)
    (:Update
      (Rendering|Material|SetScalarParameterValue (Variables|Default|GetDisintegrateMaterial) "Amount" _fadein :!class /Script/Engine.MaterialInstanceDynamic)
      (Utilities|FlowControl|Delay 0.5)
      (Input|EnableInput (stale EventOnRespawn _asplayer_controller))
      (Variables|Default|SetRespawning false))))

(event EventBeginPlay
  (Utilities|Time|SetTimerbyEvent (delegate Custom|CheckKillZServer) 1.0 true)
  (bind _returnvalue (Rendering|Material|CreateDynamicMaterialInstance (Variables|Character|GetMesh) 0 "/Game/Assets/Animations/Disintigrate_Inst.Disintigrate_Inst" "" :!class /Script/Engine.PrimitiveComponent))
  (Variables|Default|SetDisintegrateMaterial _returnvalue)
  (Utilities|Time|SetTimerbyFunctionName 0 "UpdateGroundType" 0.1 true))

(event EventOnRespawn
  (Variables|Default|SetRespawning true)
  (bind _astwo_the_edge_player_state (Utilities|Casting|CastToTwoTheEdgePlayerState (Variables|Default|GetPlayerState)))
  (bind _fadein (Timeline|Fadeout PlayFromStart)
    (:Update
      (Rendering|Material|SetScalarParameterValue (Variables|Default|GetDisintegrateMaterial) "Amount" _fadein :!class /Script/Engine.MaterialInstanceDynamic)
      (bind _asplayer_controller (Utilities|Casting|CastToPlayerController (Pawn|GetController (Variables|/Script/Engine.PlayerState|GetPawnPrivate (Variables|Default|GetPlayerState)))))
      (Input|DisableInput _asplayer_controller)
      (Utilities|FlowControl|Delay 0.5)
      (Class|TwotheEdgeCharacter|TeleportonServer (+ (.location (Variables|/Script/TwoTheEdge.TwoTheEdgePlayerState|GetLastCheckpointPos _astwo_the_edge_player_state)) "0, 0,100.000000") (.rotation (Variables|/Script/TwoTheEdge.TwoTheEdgePlayerState|GetLastCheckpointPos _astwo_the_edge_player_state)))
      (Components|Movement|StopMovementImmediately (Variables|Character|GetCharacterMovement)) ; Removes all velocity and stuff
      (CallFunction|CallServer))))

(event EventPossessed
  (params (NewController :type Controller%20Object%20Reference))
  (Utilities|FlowControl|Delay 4.0) ; Force delay to make sure BeginPlay is run
  (Class|TwotheEdgeCharacter|OnPossessed))

(event EventPossessedServer
  (CallFunction|ChangeColour)
  (Class|TwotheEdgeCharacter|CreatePlayerName))

(event EventOnGrenadeThrow
  (params (GrenadeType :type Integer%20%28by%20ref%29))
  (CallFunction|ThrowGrenade GrenadeType))

(event EventOnForwardDash
  (Animation|PlayAnimMontage "/Game/Animations/Dash_Montage.Dash_Montage" 1.0 "None"))

(event Input|ActionEvents|InputActionExplosiveGrenade
  (params (Key :type Key%20Structure :default "None"))
  (:Pressed
    (Class|TwotheEdgeCharacter|RequestGrenadeThrow (Class|KismetSystemLibrary|MakeLiteralInteger))))

(event Input|ActionEvents|InputActionFreezeGrenade
  (params (Key :type Key%20Structure :default "None"))
  (:Pressed
    (Class|TwotheEdgeCharacter|RequestGrenadeThrow (Class|KismetSystemLibrary|MakeLiteralInteger 1))))

(fn ConstructionScript
  (Variables|Default|SetExtraMovement self (Variables|Default|GetExtraMovementComponent)))

(fn ThrowGrenade
  (params (GrenadeType :type Integer))
  (bind _followcamera (Variables|Default|GetFollowCamera))
  (bind _mesh (Variables|Character|GetMesh))
  (bind _returnvalue (Transformation|GetWorldLocation _mesh))
  (bind _returnvalue_2 (Math|Vector|GetRightVector _mesh))
  (bind _returnvalue_3 (Math|Vector|GetUpVector _mesh))
  (bind _returnvalue_4 (Transformation|GetWorldRotation _followcamera))
  (bind _returnvalue_5 (* _returnvalue_2 75.0))
  (bind _returnvalue_6 (Math|Float|ClampAngle (.pitch _returnvalue_4) -5e+01 5e+01))
  (bind _returnvalue_7 (+ _returnvalue "0, 0,180.000000"))
  (bind _returnvalue_8 (* (.z _returnvalue_3) 8e+02))
  (bind _returnvalue_9 (* _returnvalue_6 5e+01))
  (bind _returnvalue_10 (+ _returnvalue_7 _returnvalue_5))
  (bind _returnvalue_11 (Math|Conversions|ToTransform(Vector) _returnvalue_10))
  (bind _returnvalue_12 (+ _returnvalue_8 _returnvalue_9))
  (bind _returnvalue_13 (Math|Float|Min(Float) _returnvalue_12 8e+02))
  (bind _returnvalue_14 (Math|Float|Max(Float) _returnvalue_13 -4e+02))
  (bind _returnvalue_15 (Math|Float|Lerp 7.5e+02 _returnvalue_14 0.5))
  (bind _returnvalue_16 (Math|Float|Max(Float) _returnvalue_15 1e+02))
  (bind _returnvalue_17 (* _returnvalue_2 _returnvalue_16))
  (bind _returnvalue_18 (Math|Vector|MakeVector (.x _returnvalue_17) (.y _returnvalue_17) _returnvalue_14))
  (switch int GrenadeType
    (:0
      (bind _returnvalue_19 (Game|SpawnActorfromClass "/Game/Blueprints/Actors/BP_ExplosionGrenade.BP_ExplosionGrenade_C" _returnvalue_11 "Undefined" 0 0))
      (Physics|SetPhysicsLinearVelocity (Variables|/Game/Blueprints/Actors/BP_ExplosionGrenade.BP_ExplosionGrenade_C|GetSphere _returnvalue_19) _returnvalue_18 false "None"))
    (:1
      (bind _returnvalue_20 (Game|SpawnActorfromClass "/Game/Blueprints/Actors/BP_FreezeGrenade.BP_FreezeGrenade_C" _returnvalue_11 "Undefined" 0 0))
      (Physics|SetPhysicsLinearVelocity (Variables|/Game/Blueprints/Actors/BP_FreezeGrenade.BP_FreezeGrenade_C|GetSphere _returnvalue_20) _returnvalue_18 false "None"))))

(fn ChangeColour
  (bind _playerstate (Variables|Default|GetPlayerState))
  (Utilities|IsValid (Variables|Default|GetDisintegrateMaterial)
    (:Is%20Valid
      (Utilities|IsValid _playerstate
        (:Is%20Valid
          (bind _astwo_the_edge_player_state (Utilities|Casting|CastToTwoTheEdgePlayerState _playerstate))
          (Rendering|Material|SetTextureParameterValue (Variables|Default|GetDisintegrateMaterial) "Emissive" (Utilities|Array|Get(acopy) (Variables|Default|GetPlayerColourTextures) (Math|Conversions|ToInteger(Byte) (Variables|/Script/TwoTheEdge.TwoTheEdgePlayerState|GetPlayerColour _astwo_the_edge_player_state))))
          (Development|PrintString (Utilities|String|ToString(Byte) (Variables|/Script/TwoTheEdge.TwoTheEdgePlayerState|GetPlayerColour _astwo_the_edge_player_state))))
        (:Is%20Not%20Valid
          (Development|PrintString "no p stHello"))))))