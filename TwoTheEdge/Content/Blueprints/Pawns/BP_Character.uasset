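; Character pawn Blueprint that makes ice floors slippery by adjusting its walking movement to the physical surface underfoot.
; A looping timer started on BeginPlay polls the current floor's surface type ten times a second.
; Each poll sets ground friction and walking braking deceleration, dropping both to zero on Ice.
; The construction script also caches the ExtraMovementComponent in the ExtraMovement variable, which this file does not otherwise use.
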(event Custom|SetGroundFriction
  (bind _charactermovement (Variables|Character|GetCharacterMovement))
  (bind _charactermovement_2 (Variables|Character|GetCharacterMovement))
  (bind _currentfloor (Variables|/Script/Engine.CharacterMovementComponent|GetCurrentFloor _charactermovement_2))
  (bind _returnvalue (Collision|GetSurfaceType (.hitresult _currentfloor)))
  (Variables|/Script/Engine.CharacterMovementComponent|SetGroundFriction _charactermovement (Utilities|Select :Index _returnvalue :SurfaceType_Default 0.8 :SurfaceType1 0.0))
  (Variables|/Script/Engine.CharacterMovementComponent|SetBrakingDecelerationWalking _charactermovement (Utilities|Select :Index _returnvalue :SurfaceType_Default 2048.0 :SurfaceType1 0.0)))

(event EventBeginPlay
  (Utilities|Time|SetTimerbyFunctionName 0 "SetGroundFriction" 0.1 true))

(fn ConstructionScript
  (Variables|Default|SetExtraMovement self (Variables|Default|GetExtraMovementComponent)))