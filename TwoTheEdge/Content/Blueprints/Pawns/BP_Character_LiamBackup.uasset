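; BP_Character_LiamBackup is a character Blueprint, apparently a backup, with grenade throwing and surface-dependent movement.
; Right mouse spawns a BP_BaseGrenade above the mesh, offset along its right vector, and launches it in an upward arc.
; A looping timer checks the floor's physical surface to set ground friction and walking braking for default, ice or tar.
; The construction script assigns the ExtraMovementComponent to the ExtraMovement variable.
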(event Custom|UpdateGroundType
  (bind _charactermovement (Variables|Character|GetCharacterMovement))
  (bind _charactermovement_2 (Variables|Character|GetCharacterMovement))
  (bind _currentfloor (Variables|/Script/Engine.CharacterMovementComponent|GetCurrentFloor _charactermovement))
  (bind _returnvalue (Collision|GetSurfaceType (.hitresult _currentfloor)))
  (Variables|/Script/Engine.CharacterMovementComponent|SetGroundFriction _charactermovement_2 (Utilities|Select :Index _returnvalue :SurfaceType_Default 0.8 :SurfaceType1 0.1 :SurfaceType2 2.0))
  (Variables|/Script/Engine.CharacterMovementComponent|SetBrakingDecelerationWalking _charactermovement_2 (Utilities|Select :Index _returnvalue :SurfaceType_Default 1.5e+03 :SurfaceType1 0.0 :SurfaceType2 5e+03)))

(event EventBeginPlay
  (Utilities|Time|SetTimerbyFunctionName 0 "UpdateGroundType" 0.1 true))

(event Input|MouseEvents|RightMouseButton
  (params (Key :type Key%20Structure :default "None"))
  (bind _mesh (Variables|Character|GetMesh))
  (bind _returnvalue (Math|Vector|GetRightVector _mesh))
  (:Pressed
    (bind _returnvalue_2 (Game|SpawnActorfromClass "/Game/Blueprints/Actors/BP_BaseGrenade.BP_BaseGrenade_C" (Math|Conversions|ToTransform(Vector) (+ (+ (Transformation|GetWorldLocation _mesh) "0, 0,180.000000") (* _returnvalue 75.0))) "Undefined" 0 0))
    (Physics|SetPhysicsLinearVelocity (Variables|/Game/Blueprints/Actors/BP_BaseGrenade.BP_BaseGrenade_C|GetSphere _returnvalue_2) (+ (* _returnvalue 7.5e+02) (* (Math|Vector|GetUpVector _mesh) 5e+02)) false "None")))

(fn ConstructionScript
  (Variables|Default|SetExtraMovement self (Variables|Default|GetExtraMovementComponent)))