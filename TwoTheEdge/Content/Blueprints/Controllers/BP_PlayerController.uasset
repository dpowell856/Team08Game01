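; Player controller that creates the local player's HUD and pause menu and handles pausing input.
; BeginPlay and Possess both call a client-side setup, guarded by an Initialised flag, that adds the HUD and a hidden, high Z-order pause widget to the player screen.
; The Pause action toggles that menu, along with the mouse cursor and the controlled pawn's input, without pausing the game itself.
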(event Custom|CallOnClient
  (if (not (Variables|Default|GetInitialised))
    (bind _returnvalue (UserInterface|CreateWidget "/Game/Blueprints/Widgets/WBP_HUD.WBP_HUD_C"))
    (UserInterface|Viewport|AddtoPlayerScreen _returnvalue)
    (bind _returnvalue_2 (UserInterface|CreateWidget "/Game/Blueprints/Widgets/WBP_PauseMenu.WBP_PauseMenu_C"))
    (bind _output_get (Variables|Default|SetPauseWidget _returnvalue_2))
    (Widget|SetVisibility _output_get "Collapsed")
    (UserInterface|Viewport|AddtoPlayerScreen _output_get 1000)
    (Variables|Default|SetInitialised true)))

(event EventBeginPlay
  (CallFunction|CallonClient))

(event EventPossess
  (params (PossessedPawn :type Pawn%20Object%20Reference))
  (CallFunction|CallonClient))

(event Input|ActionEvents|InputActionPause
  (params (Key :type Key%20Structure :default "None"))
  (bind _self self)
  (bind _pausewidget (Variables|Default|GetPauseWidget))
  (bind _returnvalue (Pawn|GetControlledPawn _self))
  (:Pressed
    (if (Widget|IsVisible _pausewidget)
      (Widget|SetVisibility _pausewidget "Collapsed")
      (Variables|Default|SetbShowMouseCursor false)
      (Input|EnableInput _returnvalue 0)
      (else
        (Widget|SetVisibility _pausewidget "Visible")
        (Variables|Default|SetbShowMouseCursor true)
        (Input|DisableInput _returnvalue 0)))))

(fn ConstructionScript)