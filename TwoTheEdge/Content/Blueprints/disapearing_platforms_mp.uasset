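; Multiplayer disappearing-platform pair where one platform, chosen at random, vanishes on contact and the other stays.
; A Character entering the Trigger calls ExecuteServer, which destroys one of the two overlap boxes, then the Trigger destroys itself.
; Overlapping a remaining box calls its DestroyOnServer event, removing that box with its cube and thruster.
; Server-named events handle all random selection and platform removal, with an IsBeingDestroyed guard against repeat selection.
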(event OnComponentBeginOverlap(Box1)
  (params (OverlappedComponent :type Primitive%20Component%20Object%20Reference) (OtherActor :type Actor%20Object%20Reference) (OtherComp :type Primitive%20Component%20Object%20Reference) (OtherBodyIndex :type Integer) (bFromSweep :type Boolean) (SweepResult :type Hit%20Result%20Structure%20%28by%20ref%29))
  (CallFunction|DestroyonServer))

(event OnComponentBeginOverlap(Box)
  (params (OverlappedComponent :type Primitive%20Component%20Object%20Reference) (OtherActor :type Actor%20Object%20Reference) (OtherComp :type Primitive%20Component%20Object%20Reference) (OtherBodyIndex :type Integer) (bFromSweep :type Boolean) (SweepResult :type Hit%20Result%20Structure%20%28by%20ref%29))
  (CallFunction|DestroyonServer2))

(event OnComponentBeginOverlap(Trigger)
  (params (OverlappedComponent :type Primitive%20Component%20Object%20Reference) (OtherActor :type Actor%20Object%20Reference) (OtherComp :type Primitive%20Component%20Object%20Reference) (OtherBodyIndex :type Integer) (bFromSweep :type Boolean) (SweepResult :type Hit%20Result%20Structure%20%28by%20ref%29))
  (Utilities|Casting|CastToCharacter OtherActor)
  (CallFunction|ExecuteServer)
  (Components|DestroyComponent (Variables|Default|GetTrigger)))

(event Custom|Destroy%20On%20Server
  (Components|DestroyComponent (Variables|Default|GetBox1))
  (Components|DestroyComponent (Variables|Default|GetCube1))
  (Components|DestroyComponent (Variables|Default|Getthruster1_0)))

(event Custom|ExecuteServer
  (if (not (or (Class|ActorComponent|IsBeingDestroyed (Variables|Default|GetBox)) (Class|ActorComponent|IsBeingDestroyed (Variables|Default|GetBox1))))
    (if (Math|Random|RandomBool)
      (Components|DestroyComponent (Variables|Default|GetBox))
      (else
        (Components|DestroyComponent (Variables|Default|GetBox1))))))

(event Custom|Destroy%20On%20Server%202
  (Components|DestroyComponent (Variables|Default|GetBox))
  (Components|DestroyComponent (Variables|Default|GetServerCube))
  (Components|DestroyComponent (Variables|Default|Getthruster)))

(fn ConstructionScript
  (|CallParentFunction))