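; Freeze grenade actor that detonates on a timer after BeginPlay and temporarily freezes characters and platforms in its blast.
; Detonation briefly expands FreezeCollider's radius from zero, then collapses it and hides the Sphere.
; The collider's overlap halts TwoTheEdgeCharacter movement or deactivates base_platform actors, restoring either after a delay.
; A character overlapping the grenade makes the Sphere extremely heavy via a mass override.
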(event OnComponentBeginOverlap(FreezeCollider)
  (params (OverlappedComponent :type Primitive%20Component%20Object%20Reference) (OtherActor :type Actor%20Object%20Reference) (OtherComp :type Primitive%20Component%20Object%20Reference) (OtherBodyIndex :type Integer) (bFromSweep :type Boolean) (SweepResult :type Hit%20Result%20Structure%20%28by%20ref%29))
  ;[1 1 1] Freeze players
  (bind _astwo_the_edge_character (Utilities|Casting|CastToTwoTheEdgeCharacter OtherActor)
    (:then
      (Development|PrintString "Frozen")
      (Pawn|Components|CharacterMovement|DisableMovement (Variables|/Script/Engine.Character|GetCharacterMovement _astwo_the_edge_character))
      (Components|Movement|StopMovementImmediately (Variables|/Script/Engine.Character|GetCharacterMovement _astwo_the_edge_character))
      (Utilities|FlowControl|Delay 4.0)
      (Development|PrintString "Unfrozen")
      (Pawn|Components|CharacterMovement|SetMovementMode (Variables|/Script/Engine.Character|GetCharacterMovement _astwo_the_edge_character) "MOVE_Walking" 0))
    (:CastFailed
      (bind _asbase_platform (Utilities|Casting|CastTobase_platform OtherActor))
      (Development|PrintString "Frozen platform")
      (Variables|/Game/Blueprints/base_platform.base_platform_C|SetActive _asbase_platform false)
      (Utilities|FlowControl|Delay 4.0)
      (Variables|/Game/Blueprints/base_platform.base_platform_C|SetActive _asbase_platform true))))

(event Custom|CustomEvent
  (Components|Activation|Activate (Variables|Default|GetParticleSystem) false)
  (Components|Sphere|SetSphereRadius (Variables|Default|GetFreeze%20Collider) 1.6e+03 true) ; Essentially enable the freeze collider
  (Utilities|FlowControl|Delay 1.0)
  (Components|Activation|Deactivate (Variables|Default|GetSphere))
  (Components|Sphere|SetSphereRadius (Variables|Default|GetFreeze%20Collider) 0.0 true)
  (Components|Activation|Deactivate (Variables|Default|GetParticleSystem))
  (Development|SetHiddeninGame (Variables|Default|GetSphere) true false))

(event Custom|Detonate
  (Components|Activation|Activate (Variables|Default|GetSphere) false)
  (Components|Sphere|SetSphereRadius (Variables|Default|GetFreeze%20Collider) 1.6e+03 true) ; Essentially enable the freeze collider
  (Utilities|FlowControl|Delay 1.0)
  (Components|Activation|Deactivate (Variables|Default|GetSphere))
  (Components|Sphere|SetSphereRadius (Variables|Default|GetFreeze%20Collider) 0.0 true)
  (Components|Activation|Deactivate (Variables|Default|GetParticleSystem))
  (Development|SetHiddeninGame (Variables|Default|GetSphere) true false))

(event EventBeginPlay
  (Utilities|Time|SetTimerbyEvent (delegate Custom|Detonate) (Variables|Default|GetDetonationDelay)))

(event Collision|EventActorBeginOverlap
  (params (OtherActor :type Actor%20Object%20Reference))
  (Utilities|Casting|CastToTwoTheEdgeCharacter OtherActor)
  (Class|PrimitiveComponent|SetMassOverrideinKg (Variables|Default|GetSphere) "None" 1e+06 true))

(fn ConstructionScript)