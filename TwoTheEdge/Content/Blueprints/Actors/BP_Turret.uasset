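; BP_Turret is a turret actor that picks and holds a target using AI Perception sight.
; UpdateTarget takes the first sight-perceived actor as CurrentTarget and timestamps the sighting, clearing the target only when enough time has passed since it was last seen.
; The construction script assigns the bullet spawn point component to BulletSpawnPoint, with no firing logic in these graphs.
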(event EventUpdateTarget
  (bind _aiperception (Variables|Default|GetAIPerception))
  (bind _outactors (Class|AIPerceptionComponent|GetPerceivedActors _aiperception "/Script/AIModule.AISense_Sight"))
  (if (> (Utilities|Array|Length _outactors) 0)
    (Variables|Default|SetCurrentTarget (Utilities|Array|Get(acopy) _outactors))
    (Variables|Default|SetTargetLastSeen (Math|DateTime|UTCNow))
    (elif (>= (- (Math|DateTime|UTCNow) (Variables|Default|GetTargetLastSeen)) "")
      (Variables|Default|SetCurrentTarget 0))))

(fn ConstructionScript
  (Variables|Default|SetBulletSpawnPoint (Variables|Default|GetBullet%20Spawn%20Point%20Comp)))