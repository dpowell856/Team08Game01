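; BP_FinishTrigger is a finish trigger actor that records players completing the course and announces their placing.
; On overlap with a TwoTheEdgeCharacter, it checks the player state's Finished flag so each player counts only once.
; A first finish activates a particle system, prints the player's name with the game state's NextWinPosition, sets Finished and increments that position for the next player.
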(event EventBeginPlay)

(event Collision|EventActorBeginOverlap
  (params (OtherActor :type Actor%20Object%20Reference))
  (bind _astwo_the_edge_character (Utilities|Casting|CastToTwoTheEdgeCharacter OtherActor))
  (bind _astwo_the_edge_player_state (Utilities|Casting|CastToTwoTheEdgePlayerState (Variables|/Script/Engine.Pawn|GetPlayerState _astwo_the_edge_character)))
  (bind _astwo_the_edge_game_state (Utilities|Casting|CastToTwoTheEdgeGameState (Game|GetGameState)))
  (if (not (Variables|/Script/TwoTheEdge.TwoTheEdgePlayerState|GetFinished _astwo_the_edge_player_state))
    (Components|Activation|Activate (Variables|Default|GetParticleSystem) true)
    (Development|PrintString (Utilities|String|ToString(Text) (Utilities|Text|FormatText "{PlayerName} placed position {Position}" (PlayerState|GetPlayerName _astwo_the_edge_player_state) (Variables|/Script/TwoTheEdge.TwoTheEdgeGameState|GetNextWinPosition _astwo_the_edge_game_state))))
    (Variables|/Script/TwoTheEdge.TwoTheEdgePlayerState|SetFinished _astwo_the_edge_player_state true)
    (Math|Integer|IncrementInt (Variables|/Script/TwoTheEdge.TwoTheEdgeGameState|GetNextWinPosition _astwo_the_edge_game_state))))

(fn ConstructionScript)