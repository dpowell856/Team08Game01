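; Pulsing laser hazard actor that respawns a player character caught in its line of fire.
; BeginPlay sets the particle beam endpoints between two static meshes, with an offset at the source, and starts a looping timer that calls LaserOn.
; Each pulse shows the beam, makes a single Visibility trace from the Box to the end mesh, respawns any hit BP_Character not already respawning, then hides the beam after a short delay.
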(event Custom|LaserOn
  (Rendering|SetVisibility (Variables|Default|GetParticleSystem) true false)
  (bind _outhit (Collision|LineTraceByChannel (Transformation|GetWorldLocation (Variables|Default|GetBox)) (Transformation|GetWorldLocation (Variables|Default|GetStaticMesh1)) "TraceTypeQuery1" false 0 "None"))
  (Utilities|FlowControl|Sequence
    (:then_0
      (bind _asbp_character (Utilities|Casting|CastToBP_Character (.hitactor _outhit)))
      (if (not (Variables|/Game/Blueprints/Pawns/BP_Character_New.BP_Character_C|GetRespawning _asbp_character))
        (Class|TwotheEdgeCharacter|Respawn _asbp_character)))
    (:then_1
      (Utilities|FlowControl|Delay 0.25)
      (Rendering|ToggleVisibility (Variables|Default|GetParticleSystem) false))))

(event EventBeginPlay
  (bind _particlesystem (Variables|Default|GetParticleSystem))
  (Utilities|Time|SetTimerbyFunctionName 0 "LaserOn" 2.0 true)
  (Class|ParticleSystemComponent|SetBeamSourcePoint _particlesystem 0 (- (Transformation|GetWorldLocation (Variables|Default|GetStaticMesh)) (Variables|Default|GetLaserStartPlacement)))
  (Class|ParticleSystemComponent|SetBeamTargetPoint _particlesystem 0 (Transformation|GetWorldLocation (Variables|Default|GetStaticMesh1))))

(event Collision|EventActorBeginOverlap
  (params (OtherActor :type Actor%20Object%20Reference)))

(fn ConstructionScript)