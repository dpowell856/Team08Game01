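; Stamina pickup actor that adds a fixed amount of stamina to the collecting character's TwoTheEdgePlayerState.
; Its box overlap forwards the other actor to OnOverlap, while the OnPickup event casts the character's player state and grants the stamina.
; It then removes the sphere component, activates a particle effect and waits briefly before destroying itself, keeping this in the event graph because functions cannot contain Delay.
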(event OnComponentBeginOverlap(Box)
  (params (OverlappedComponent :type Primitive%20Component%20Object%20Reference) (OtherActor :type Actor%20Object%20Reference) (OtherComp :type Primitive%20Component%20Object%20Reference) (OtherBodyIndex :type Integer) (bFromSweep :type Boolean) (SweepResult :type Hit%20Result%20Structure%20%28by%20ref%29))
  (Class|Pickup|OnOverlap OtherActor))

(event EventBeginPlay)

(event Collision|EventActorBeginOverlap
  (params (OtherActor :type Actor%20Object%20Reference)))

(event EventTick
  (params (DeltaSeconds :type Float%20%28single-precision%29)))

(event EventOnPickup
  (params (Character :type Two%20the%20Edge%20Character%20Object%20Reference))
  (bind _astwo_the_edge_player_state (Utilities|Casting|CastToTwoTheEdgePlayerState (Variables|/Script/Engine.Pawn|GetPlayerState Character)))
  (Class|TwotheEdgePlayerState|AddStamina _astwo_the_edge_player_state 3.0)
  ;[1 1 1] Destroy-y stuff - would put in a function but can't put Delay in function
  (Components|DestroyComponent (Variables|Default|GetSphere))
  ;;[1 1 1] Creates particle effects before finally destroying
  (Components|Activation|Activate (Variables|Default|GetParticleSystem) false)
  (Utilities|FlowControl|Delay 1.0)
  (Actor|DestroyActor))

(fn ConstructionScript)