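; Grenade actor that explodes on a timer after it spawns.
; BeginPlay starts a one-shot timer using DetonationDelay; on detonation the sphere is destroyed, the particle system and radial force activate, and the actor destroys itself after a short delay.
; Overlapping a TwoTheEdgeCharacter overrides the sphere's mass to an extremely high value.
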(event Custom|Detonate
  (Components|DestroyComponent (Variables|Default|GetSphere))
  (Components|Activation|Activate (Variables|Default|GetParticleSystem) false)
  (Components|Activation|Activate (Variables|Default|GetRadialForce) false)
  (Utilities|FlowControl|Delay 0.2)
  (Actor|DestroyActor))

(event EventBeginPlay
  (Utilities|Time|SetTimerbyEvent (delegate Custom|Detonate) (Variables|Default|GetDetonationDelay)))

(event Collision|EventActorBeginOverlap
  (params (OtherActor :type Actor%20Object%20Reference))
  (Utilities|Casting|CastToTwoTheEdgeCharacter OtherActor)
  (Class|PrimitiveComponent|SetMassOverrideinKg (Variables|Default|GetSphere) "None" 1e+06 true))

(fn ConstructionScript)