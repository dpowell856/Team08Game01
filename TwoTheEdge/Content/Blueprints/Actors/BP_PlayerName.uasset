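; BP_PlayerName is an actor that displays a name as world-space text, apparently a player name label.
; The construction script applies the Name variable to the text render component.
; Every tick it rotates its root to face the first player's camera, creating a billboard effect that keeps the text facing the viewer.
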(event EventBeginPlay)

(event Collision|EventActorBeginOverlap
  (params (OtherActor :type Actor%20Object%20Reference)))

(event EventTick
  (params (DeltaSeconds :type Float%20%28single-precision%29)))

(event EventOnTick
  ;[1 1 1] Rotates towards the camera (Billboard effect)
  (Transformation|SetWorldRotation (Variables|Default|GetDefaultSceneRoot) (Math|Rotator|MakeRotfromX (Math|Vector|Normalize (- (Camera|GetCameraLocation (Game|GetPlayerCameraManager 0)) (Transformation|GetActorLocation)))) false false))

(fn ConstructionScript
  (Variables|Default|SetTextRenderComponent (Variables|Default|GetName)))