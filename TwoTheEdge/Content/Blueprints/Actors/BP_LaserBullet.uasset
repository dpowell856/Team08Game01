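; BP_LaserBullet is a laser projectile that respawns a locally controlled TwoTheEdgeCharacter it hits.
; On a Shape hit it branches on net mode into client and server events, which currently share identical logic.
; The bullet destroys itself after any hit or when its lifetime is exceeded.
; The construction script assigns Shape as ProjectileMesh and sets ProjectileMovement to None.
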(event OnComponentHit(Shape)
  (params (HitComponent :type Primitive%20Component%20Object%20Reference) (OtherActor :type Actor%20Object%20Reference) (OtherComp :type Primitive%20Component%20Object%20Reference) (NormalImpulse :type Vector :default "0, 0, 0") (Hit :type Hit%20Result%20Structure%20%28by%20ref%29))
  (bind _returnvalue (Class|Bullet|GetNetMode))
  (if (== _returnvalue 3)
    (CallFunction|OnHitClient OtherActor)
    (else
      (CallFunction|OnHitServer OtherActor))))

(event Custom|OnHitServer
  (params (Actor%20Hit :type Actor%20Object%20Reference))
  (bind _astwo_the_edge_character (Utilities|Casting|CastToTwoTheEdgeCharacter Actor%20Hit)
    (:then
      (if (Pawn|IsLocallyControlled _astwo_the_edge_character)
        (Class|TwotheEdgeCharacter|Respawn _astwo_the_edge_character)))
    (:CastFailed
      _))
  (Actor|DestroyActor))

(event Custom|OnHitClient
  (params (Actor%20Hit :type Actor%20Object%20Reference))
  (bind _astwo_the_edge_character (Utilities|Casting|CastToTwoTheEdgeCharacter Actor%20Hit)
    (:then
      (if (Pawn|IsLocallyControlled _astwo_the_edge_character)
        (Class|TwotheEdgeCharacter|Respawn _astwo_the_edge_character)))
    (:CastFailed
      _))
  (Actor|DestroyActor))

(event EventOnLifetimeExceeded
  (Actor|DestroyActor))

(fn ConstructionScript
  (Variables|Default|SetProjectileMovement 0)
  (Variables|Default|SetProjectileMesh (Variables|Default|GetShape)))