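; Freeze grenade pickup actor that adds one freeze grenade to the collecting character's TwoTheEdgePlayerState.
; Box overlaps are passed to OnOverlap, and the OnPickup event attempts the add.
; A successful add hides the visuals, removes the lights and sphere, then destroys the actor immediately, as the delayed particle effect is disconnected.
; Tick turns the paper sprite toward the player camera as a billboard.
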(event OnComponentBeginOverlap(Box)
  (params (OverlappedComponent :type Primitive%20Component%20Object%20Reference) (OtherActor :type Actor%20Object%20Reference) (OtherComp :type Primitive%20Component%20Object%20Reference) (OtherBodyIndex :type Integer) (bFromSweep :type Boolean) (SweepResult :type Hit%20Result%20Structure%20%28by%20ref%29))
  (Class|Pickup|OnOverlap OtherActor))

(event EventBeginPlay)

(event Collision|EventActorBeginOverlap
  (params (OtherActor :type Actor%20Object%20Reference)))

(event EventTick
  (params (DeltaSeconds :type Float%20%28single-precision%29))
  (bind _returnvalue (Game|GetPlayerCameraManager 0))
  (bind _papersprite (Variables|Default|GetPaperSprite))
  (bind _returnvalue_2 (Transformation|GetWorldLocation _papersprite))
  (bind _returnvalue_3 (Camera|GetCameraLocation _returnvalue))
  (bind _returnvalue_4 (- _returnvalue_3 _returnvalue_2))
  (bind _returnvalue_5 (Math|Vector|Normalize _returnvalue_4))
  (bind _returnvalue_6 (Math|Rotator|MakeRotfromX _returnvalue_5))
  ;[1 1 1] Rotates towards the camera (Billboard effect)
  (Transformation|SetWorldRotation (Variables|Default|GetPaperSprite) (Math|Rotator|MakeRotator (.roll _returnvalue_6) (.pitch _returnvalue_6) (+ (.yaw _returnvalue_6) -9e+01)) false false))

(event EventOnPickup
  (params (Character :type Two%20the%20Edge%20Character%20Object%20Reference))
  (bind _astwo_the_edge_player_state (Utilities|Casting|CastToTwoTheEdgePlayerState (Variables|/Script/Engine.Pawn|GetPlayerState Character)))
  (bind _returnvalue (Class|TwotheEdgePlayerState|AddFreezeGrenades _astwo_the_edge_player_state 1))
  (if _returnvalue
    (Development|SetHiddeninGame (Variables|Default|GetCylinder) true false)
    (Development|SetHiddeninGame (Variables|Default|GetPaperSprite) true false)
    (Components|DestroyComponent (Variables|Default|GetLight1))
    ;[1 1 1] Destroy-y stuff - would put in a function but can't put Delay in function
    (Components|DestroyComponent (Variables|Default|GetLight))
    (Components|DestroyComponent (Variables|Default|GetSphere))
    ;;[1 1 1] Creates particle effects before finally destroying
    (Actor|DestroyActor)))

(fn ConstructionScript)